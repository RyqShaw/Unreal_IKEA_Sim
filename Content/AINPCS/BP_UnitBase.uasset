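; BP_UnitBase is a base AI controller for NPC units that runs a behavior tree and spots customer units by sight.
; BeginPlay starts BTAsset, and AI perception updates feed HandleSightSense.
; That function filters for sight stimuli from actors whose class is exactly BP_CustomerUnit, then writes the actor to the TargetObject blackboard key.
; It does not check whether sight was gained or lost and never clears the key.
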(event `self.ReceiveBeginPlay`
  (`self.RunBehaviorTree` (`self.BTAsset`)))

(event `self.AIPerception.OnTargetPerceptionUpdated`
  (params (Actor :type "Actor Object Reference") (Stimulus :type "AIStimulus Structure"))
  (`self.HandleSightSense` Actor Stimulus))

(fn `HandleSightSense`
  (params (Actor :type "Actor Object Reference") (Stimulus :type "AIStimulus Structure"))
  (bind _returnvalue (`AIPerceptionSystem.GetSenseClassForStimulus` Stimulus))
  (if (== _returnvalue "/Script/AIModule.AISense_Sight")
    (if (== (`GameplayStatics.GetObjectClass` (`local.Actor`)) "/Game/AINPCS/Customer/BP_CustomerUnit.BP_CustomerUnit_C")
      (`BlackboardComponent.SetValueAsObject` (`AIBlueprintHelperLibrary.GetBlackboard` null) "TargetObject" (`local.Actor`))
      (else
        (return)))
    (else
      (return))))

(fn `UserConstructionScript`)