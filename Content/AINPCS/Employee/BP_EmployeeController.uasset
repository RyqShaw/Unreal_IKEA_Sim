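; AI controller for employee NPCs that runs BT_Employee on possession and seeds the blackboard with the pawn's EmployeeState.
; UpdateStateInBlackboard writes state changes to the blackboard.
; FindNearestPatrolPath scans all BP_PatrolPoint actors and stores the closest as CurrentPatrolPoint.
; Tick clears that patrol point whenever the employee's state differs from one specific enum value.
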(event `self.ReceiveBeginPlay`
  (set `self.BTAsset` "/Game/AINPCS/Employee/BT_Employee.BT_Employee")
  (`parent.ReceiveBeginPlay`))

(event `self.ReceivePossess`
  (params (PossessedPawn :type "Pawn Object Reference"))
  (`self.RunBehaviorTree` "/Game/AINPCS/Employee/BT_Employee.BT_Employee")
  (bind _asbp_employee_unit (cast `/Game/AINPCS/Employee/BP_EmployeeUnit` PossessedPawn))
  (`BlackboardComponent.SetValueAsEnum` (`AIBlueprintHelperLibrary.GetBlackboard` PossessedPawn) "EmployeeState" (`/Game/AINPCS/Employee/BP_EmployeeUnit.EmployeeState` _asbp_employee_unit)))

(event `self.ReceiveTick`
  (params (DeltaSeconds :type "Float (single-precision)"))
  (bind _asbp_employee_unit (cast `/Game/AINPCS/Employee/BP_EmployeeUnit` (`self.K2_GetPawn`)))
  (if (not (`|EnumEquality` (`/Game/AINPCS/Employee/BP_EmployeeUnit.EmployeeState` _asbp_employee_unit) "NewEnumerator2"))
    (`BlackboardComponent.SetValueAsObject` (`AIBlueprintHelperLibrary.GetBlackboard` null) "CurrentPatrolPoint" null)))

(fn `FindNearestPatrolPath`
  (set `self.ClosestDistance` 999999.0)
  (bind _outactors (`GameplayStatics.GetAllActorsOfClass` "/Game/AINPCS/Patrol/BP_PatrolPoint.BP_PatrolPoint_C"))
  (for _array_element _outactors
    (bind _returnvalue (`KismetMathLibrary.Vector_Distance` (`self.K2_GetActorLocation` (`self.K2_GetPawn`)) (`self.K2_GetActorLocation` _array_element)))
    (if (< _returnvalue (`self.ClosestDistance`))
      (set `self.ClosestDistance` _returnvalue)
      (set `self.ClosestPathPoint` _array_element)))
  (`BlackboardComponent.SetValueAsObject` (`AIBlueprintHelperLibrary.GetBlackboard` null) "CurrentPatrolPoint" (`self.ClosestPathPoint`)))

(fn `UpdateStateInBlackboard`
  (params (NewState :type "/Game/AINPCS/Employee/E_EmployeeState Enum" :default "NewEnumerator0"))
  (`BlackboardComponent.SetValueAsEnum` (`AIBlueprintHelperLibrary.GetBlackboard` null) "EmployeeState" NewState))

(fn `UserConstructionScript`
  (`parent.UserConstructionScript`))