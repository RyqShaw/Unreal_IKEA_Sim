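; BP_EmployeeUnit is an AI-controlled employee unit with an overhead or attached UI widget.
; On BeginPlay it hands itself to its WBG_EmployeeUI widget, and every Tick rotates that widget component to face the player camera.
; SetEmployeeState stores the new state and forwards it to BP_EmployeeController to update the Blackboard.
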(event `self.ReceiveBeginPlay`
  (bind _aswbg_employee_ui (cast `/Game/AINPCS/Employee/WBG_EmployeeUI` (`WidgetComponent.GetUserWidgetObject` (`self.Widget`))))
  (set `/Game/AINPCS/Employee/WBG_EmployeeUI.EmployeeRef` self _aswbg_employee_ui))

(event `self.ReceiveTick`
  (params (DeltaSeconds :type "Float (single-precision)"))
  (`SceneComponent.K2_SetWorldRotation` (`self.Widget`) (`KismetMathLibrary.MakeRotator` (.roll (`KismetMathLibrary.FindLookAtRotation` (`SceneComponent.K2_GetComponentLocation` (`self.Widget`)) (`PlayerCameraManager.GetCameraLocation` (`GameplayStatics.GetPlayerCameraManager` 0)))) (.pitch (`KismetMathLibrary.FindLookAtRotation` (`SceneComponent.K2_GetComponentLocation` (`self.Widget`)) (`PlayerCameraManager.GetCameraLocation` (`GameplayStatics.GetPlayerCameraManager` 0)))) (.yaw (`KismetMathLibrary.FindLookAtRotation` (`SceneComponent.K2_GetComponentLocation` (`self.Widget`)) (`PlayerCameraManager.GetCameraLocation` (`GameplayStatics.GetPlayerCameraManager` 0))))) false false))

(fn `SetEmployeeState`
  (params (State :type "/Game/AINPCS/Employee/E_EmployeeState Enum" :default "NewEnumerator0"))
  (bind _output_get (set `self.EmployeeState` State))
  (bind _asbp_employee_controller (cast `/Game/AINPCS/Employee/BP_EmployeeController` (`self.GetController`)))
  (`/Game/AINPCS/Employee/BP_EmployeeController.UpdateStateInBlackboard` _asbp_employee_controller _output_get))

(fn `UserConstructionScript`
  (`parent.UserConstructionScript`))