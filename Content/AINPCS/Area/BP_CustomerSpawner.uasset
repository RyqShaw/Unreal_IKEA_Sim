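; BP_CustomerSpawner is an actor that repeatedly spawns BP_CustomerUnit at its own location during waves.
; A self-recursive Spawn event loops on a random delay between frequency bounds, spawning only while Enabled and BP_StrategyGameMode reports InWave.
; The loop keeps polling when those conditions fail, but stops if the game mode cast fails.
; BeginPlay starts the loop and also adds a WBP_Score widget to the viewport.
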(event `self.ReceiveBeginPlay`
  (`self.Spawn`)
  (bind _returnvalue (`|CreateWidget` "/Game/Variant_Strategy/Blueprints/WBP_Score.WBP_Score_C"))
  (`UserWidget.SetDesiredSizeInViewport` _returnvalue (100.0 50.0))
  (`UserWidget.AddToViewport` _returnvalue 0))

(event `self.ReceiveTick`
  (params (DeltaSeconds :type "Float (single-precision)")))

(event `Spawn`
  (bind _asbp_strategy_game_mode (cast `/Game/Variant_Strategy/Blueprints/BP_StrategyGameMode` (`GameplayStatics.GetGameMode`)))
  (if (and (`self.Enabled`) (`/Game/Variant_Strategy/Blueprints/BP_StrategyGameMode.InWave` _asbp_strategy_game_mode))
    (cast `/Game/Variant_Strategy/Blueprints/BP_StrategyGameMode` (`GameplayStatics.GetGameMode`))
    (`|SpawnActorFromClass` "/Game/AINPCS/Customer/BP_CustomerUnit.BP_CustomerUnit_C" (`KismetMathLibrary.MakeTransform` (`self.K2_GetActorLocation`)) "AdjustIfPossibleButAlwaysSpawn" "MultiplyWithRoot" null null))
  (`KismetSystemLibrary.Delay` (`KismetMathLibrary.RandomFloatInRange` (`self.SpawnFrequencyLower`) (`self.SpawnFrequencyUpper`)))
  (`self.Spawn`))

(fn `UserConstructionScript`)