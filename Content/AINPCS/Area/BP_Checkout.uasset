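; BP_Checkout is a checkout area that charges NPC customers for the items they hold.
; Each tick it scans all BP_EmployeeUnit actors and sets IsStaffed once any is in a particular employee state, never clearing it here.
; The Checkout function deducts item count times CostPerItem from a valid customer's money and empties their held items, only if they can afford the total; it does not check IsStaffed.
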(event `self.ReceiveTick`
  (params (DeltaSeconds :type "Float (single-precision)"))
  (bind _outactors (`GameplayStatics.GetAllActorsOfClass` "/Game/AINPCS/Employee/BP_EmployeeUnit.BP_EmployeeUnit_C"))
  (for _array_element _outactors
    (if (`|EnumEquality` (`/Game/AINPCS/Employee/BP_EmployeeUnit.EmployeeState` _array_element) "NewEnumerator1")
      (set `self.IsStaffed` true)
      (break))))

(fn `Checkout`
  (params (Customer :type "/Game/AINPCS/Customer/BP_CustomerUnit Object Reference"))
  (bind _money (`/Game/AINPCS/Customer/BP_CustomerUnit.Money` Customer))
  (bind _returnvalue (* (`/Game/AINPCS/Customer/BP_CustomerUnit.ItemsHeld` Customer) (`self.CostPerItem`)))
  (if (`KismetSystemLibrary.IsValid` Customer)
    (if (>= _money _returnvalue)
      (set `/Game/AINPCS/Customer/BP_CustomerUnit.Money` (- _money _returnvalue) Customer)
      (set `/Game/AINPCS/Customer/BP_CustomerUnit.ItemsHeld` 0 Customer))))

(fn `UserConstructionScript`)